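; BP_Tank is the tank Blueprint, turning player input into movement, camera aiming and firing.
; On BeginPlay it hands the barrel, turret and tracks to the TankAiming and TankMovement components and registers itself with its HealthBarUI widget.
; Move and turn axes feed TankMovement, while separate throttle axes drive each track directly.
; Fire calls TankAiming, and aim axes rotate an azimuth gimbal and camera, scaled by delta time.
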(event EventBeginPlay
  (Class|TankAimingComponent|Ininitialise (Variables|Default|GetTankAiming) (Variables|Default|GetTankBarrel) (Variables|Default|GetTankTurret))
  (Class|TankMovementComponent|Ininitialise (Variables|Default|GetTankMovement) (Variables|Default|GetTankTrackL) (Variables|Default|GetTankTrackR))
  (bind _ashealth_bar_ui (Utilities|Casting|CastToHealthBarUI (UserInterface|GetUserWidgetObject (Variables|Default|GetWidget))))
  (Variables|/Game/UI/HealthBarUI.HealthBarUI_C|SetTank _ashealth_bar_ui self))

(event Collision|EventActorBeginOverlap
  (params (OtherActor :type Actor%20Object%20Reference)))

(event Input|ActionEvents|InputActionFire
  (params (Key :type Key%20Structure))
  ;[1 1 1] Fire controll
  (:Pressed
    (Class|TankAimingComponent|Fire (Variables|Default|GetTankAiming))))

(event Input|AxisEvents|InputAxisAimAzimuth
  (params (AxisValue :type Float%20%28single-precision%29))
  ;[1 1 1] Camera input binding
  (Transformation|AddLocalRotation (Variables|Default|GetAzimuthGimbal) (Math|Rotator|MakeRotator 0.0 0.0 (* AxisValue (Utilities|Time|GetWorldDeltaSeconds) 1e+02)) false false))

(event Input|AxisEvents|InputAxisIntendMoveForvard
  (params (AxisValue :type Float%20%28single-precision%29))
  (Class|TankMovementComponent|IntendMoveForvard (Variables|Default|GetTankMovement) AxisValue))

(event Input|AxisEvents|InputAxisLeftTrackThrottle
  (params (AxisValue :type Float%20%28single-precision%29))
  (Class|TankTrack|SetThrottle (Variables|Default|GetTankTrackL) AxisValue))

(event Input|AxisEvents|InputAxisIntendMoveBackward
  (params (AxisValue :type Float%20%28single-precision%29))
  (Class|TankMovementComponent|IntendMoveForvard (Variables|Default|GetTankMovement) (* AxisValue -1.0)))

(event Input|AxisEvents|InputAxisRightTrackThrottle
  (params (AxisValue :type Float%20%28single-precision%29))
  (Class|TankTrack|SetThrottle (Variables|Default|GetTankTrackR) AxisValue))

(event Input|AxisEvents|InputAxisAimElevation
  (params (AxisValue :type Float%20%28single-precision%29))
  ;[1 1 1] Camera input binding
  (Transformation|AddLocalRotation (Variables|Default|GetCamera) (Math|Rotator|MakeRotator 0.0 (* AxisValue (Utilities|Time|GetWorldDeltaSeconds) 1e+02) 0.0) false false))

(event Input|AxisEvents|InputAxisIntendTurnLeft
  (params (AxisValue :type Float%20%28single-precision%29))
  (Class|TankMovementComponent|IntendTurnLeft (Variables|Default|GetTankMovement) AxisValue))

(event Input|AxisEvents|InputAxisIntendTurnRight
  (params (AxisValue :type Float%20%28single-precision%29))
  (Class|TankMovementComponent|IntendTurnRight (Variables|Default|GetTankMovement) AxisValue))

(fn ConstructionScript)